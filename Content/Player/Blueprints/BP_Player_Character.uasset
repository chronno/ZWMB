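; Player character Blueprint that handles running, crouching, jumping and vaulting over obstacles.
; Jump input has ParkourComponent search for parkour elements, with a no-object event falling back to a normal jump.
; Vault events pass three path points to the component for a motion-warped montage, stopping the vault on completion.
; RPC-named events relay run and vault actions, run toggles walk speed, and a crouch timeline lengthens the camera boom.
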(event Custom|RPC%20Vault
  (params (StartingPoint :type Vector) (MiddlePoint :type Vector) (EndPoint :type Vector))
  ;[1 1 1] OnVault
  (CallFunction|ExecuteVault StartingPoint MiddlePoint EndPoint))

(event Custom|NoObjectDetected
  ;[1 1 1] Detect Objects for Jump
  ;;[1 1 1] No Object Detected
  (Character|Jump))

(event Custom|ExecuteVault
  (params (StartingPoint :type Vector) (MiddlePoint :type Vector) (EndPoint :type Vector))
  ;[1 1 1] OnVault
  (Default|StartVaultingAnimation (Variables|Default|GetParkour%20Component) (Variables|Default|GetMotionWarping) (Transformation|GetActorRotation) StartingPoint MiddlePoint EndPoint (Variables|Character|GetCharacterMovement))
  (Animation|Montage|PlayMontage (Variables|Character|GetMesh) "/Game/Player/Animations/MM_VaultOver_Montage.MM_VaultOver_Montage"
    (:OnCompleted
      (Default|StopVaultingAnimation (Variables|Default|GetParkour%20Component) (Variables|Character|GetCharacterMovement)))))

(event Custom|RCP%20Run
  (params (IsRunning :type Boolean))
  ;[1 1 1] Run
  (CallFunction|ToggleRun IsRunning))

(event Custom|ToggleRun
  (params (IsRunning :type Boolean))
  ;[1 1 1] Run
  (CallFunction|UpdateCharacterMovementSpeed IsRunning))

(event Input|EnhancedActionEvents|EnhancedInputActionIA_Run
  (params (ActionValue :type Boolean) (ElapsedSeconds :type Float%20%28double-precision%29) (TriggeredSeconds :type Float%20%28double-precision%29) (InputAction :type Input%20Action%20Object%20Reference :default "/Game/Player/Input/Actions/IA_Run.IA_Run"))
  ;[1 1 1] Run
  (:Triggered
    (CallFunction|RCPRun ActionValue :!label _label))
  (:Completed
    (goto _label)))

(event Input|EnhancedActionEvents|EnhancedInputActionIA_Crouch
  (params (ActionValue :type Boolean) (ElapsedSeconds :type Float%20%28double-precision%29) (TriggeredSeconds :type Float%20%28double-precision%29) (InputAction :type Input%20Action%20Object%20Reference :default "/Game/Player/Input/Actions/IA_Crouch.IA_Crouch"))
  ;[1 1 1] Crouch
  (:Started
    (Character|Crouch)
    (bind _lenght (Timeline|CrouchCameraAnimation PlayFromStart)
      (:Update
        (Variables|/Script/Engine.SpringArmComponent|SetTargetArmLength (Variables|Default|GetCameraBoom) (Math|Float|Lerp 4e+02 5e+02 _lenght)))))
  (:Completed
    (Character|UnCrouch)
    (Timeline|CrouchCameraAnimation ReverseFromEnd)))

(event Input|EnhancedActionEvents|EnhancedInputActionIA_Jump
  (params (ActionValue :type Boolean) (ElapsedSeconds :type Float%20%28double-precision%29) (TriggeredSeconds :type Float%20%28double-precision%29) (InputAction :type Input%20Action%20Object%20Reference :default "/Game/Player/Input/Actions/IA_Jump.IA_Jump"))
  ;[1 1 1] Detect Objects for Jump
  (:Started
    (Default|SearchParkourElement (Variables|Default|GetParkour%20Component)))
  (:Completed
    (if (Variables|Default|GetbWasJumping)
      (Character|StopJumping))))

(event EventBeginPlay)

(event Collision|EventActorBeginOverlap
  (params (OtherActor :type Actor%20Object%20Reference)))

(event EventTick
  (params (DeltaSeconds :type Float%20%28single-precision%29)))

(fn ConstructionScript
  (CallFunction|UpdateCharacterMovementSpeed false))

(fn UpdateCharacterMovementSpeed
  (params (Running :type Boolean))
  (if Running
    (Variables|/Script/Engine.CharacterMovementComponent|SetMaxWalkSpeed (Variables|Character|GetCharacterMovement) (LocalVariables|GetRunSpeed))
    (else
      (Variables|/Script/Engine.CharacterMovementComponent|SetMaxWalkSpeed (Variables|Character|GetCharacterMovement) (LocalVariables|GetWalkSpeed)))))